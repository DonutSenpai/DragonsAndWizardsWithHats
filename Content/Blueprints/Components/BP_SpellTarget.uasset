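; BP_SpellTarget is a spell target Blueprint that keeps its Sphere component sized to match the radius of its SpellCollision sphere.
; The construction script converts the collision radius into a uniform diameter-based relative scale, assuming a 100-unit base sphere.
; BeginPlay reapplies the same scale after a very short delay, and Tick is unused.
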(event EventBeginPlay
  (Utilities|FlowControl|Delay 0.01)
  (Transformation|SetRelativeScale3D (Variables|Default|GetSphere) (Math|Conversions|ToVector(Float) (* (/ (Variables|/Script/Engine.SphereComponent|GetSphereRadius (Variables|Default|GetSpellCollision)) 1e+02) 2.0))))

(event EventTick
  (params (DeltaSeconds :type Float%20%28single-precision%29)))

(fn ConstructionScript
  (Transformation|SetRelativeScale3D (Variables|Default|GetSphere) (Math|Conversions|ToVector(Float) (* (/ (Variables|/Script/Engine.SphereComponent|GetSphereRadius (Variables|Default|GetSpellCollision)) 1e+02) 2.0))))