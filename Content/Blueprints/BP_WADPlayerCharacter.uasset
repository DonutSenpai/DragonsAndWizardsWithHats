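; Player character Blueprint for a multiplayer spellcasting mage, with a timed sprint, a brief casting flag and spell slots filled in the construction script.
; HealthComponent events drive orb color, replicated through RPCs and a RepNotify, and pop the hat off at quarter health.
; Death hides the mesh, drops hat and staff as physics objects, spawns a spirit and fades in a local post-process saturation effect; resurrection reverses this.
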(event OnHealthChanged(HealthComponent)
  (params (ChangeValue :type Float%20%28single-precision%29) (InstigatingActor :type Actor%20Object%20Reference))
  (Utilities|FlowControl|Sequence
    (:then_0
      (switch Utilities|FlowControl|Switch|SwitchonEHealthStateEnum (Variables|/Script/WizardsAndDragons.WADHealthComponent|GetHealthStateEnum (Variables|Default|GetHealthComponent))
        (:HE_FullHealth
          (Cosmetics|ResetHat :!label _label))
        (:HE_ThreeQuarterHealth
          (goto _label))
        (:HE_QuarterHealth
          (bind _successfully_detached (Cosmetics|DetachHat))
          (Cosmetics|AddHatForce _successfully_detached))))
    (:then_1
      (CallFunction|ChangeOrbColor (Utilities|Select :Index (Variables|/Script/WizardsAndDragons.WADHealthComponent|GetHealthStateEnum (Variables|Default|GetHealthComponent)) :HE_FullHealth "(R=0.187448,G=1.000000,B=0.024608,A=1.000000)" :HE_ThreeQuarterHealth "(R=0.955831,G=1.000000,B=0.000000,A=1.000000)" :HE_HalfHealth "(R=1.000000,G=0.438857,B=0.016962,A=1.000000)" :HE_QuarterHealth "(R=1.000000,G=0.000000,B=0.009744,A=1.000000)" :HE_NoHealth "(R=0.000000,G=0.000000,B=0.000000,A=0.856000)")))))

(event OnDeath(HealthComponent)
  ;[1 1 1] On Death Event in Player
  (Utilities|FlowControl|Sequence
    (:then_0
      (Rendering|SetVisibility (Variables|Default|GetOrbEffect) false false)
      (Collision|SetCollisionResponsetoChannel (Variables|Default|GetCapsuleComponent) "ECC_Pawn" "ECR_Overlap")
      (Rendering|SetVisibility (Variables|Character|GetMesh) false false)
      (CallFunction|HatStaffonDeathAnimation)
      (Class|WizardsandDragonsCharacter|SetInputDisabled)
      (bind _returnvalue (Game|SpawnActorfromClass "/Game/Blueprints/Effects/BP_DeathSpiritEffect.BP_DeathSpiritEffect_C" (Math|Transform|MakeTransform (Transformation|GetWorldLocation (Variables|Default|GetCapsuleComponent)) "0, 0, 0" "1,1,1") "AlwaysSpawn" 0 0))
      (Variables|Default|SetDeathSpirit _returnvalue)
      (CallFunction|FadeinDeathPostProcess true))))

(event OnResurrect(HealthComponent)
  (CallFunction|OnResurrectHatandStaff)
  (Actor|DestroyActor (Variables|Default|GetDeathSpirit))
  (Rendering|SetVisibility (Variables|Default|GetOrbEffect) true false)
  (Collision|SetCollisionResponsetoChannel (Variables|Default|GetCapsuleComponent) "ECC_Pawn" "ECR_Block")
  (Rendering|SetVisibility (Variables|Character|GetMesh) true false)
  (CallFunction|FadeinDeathPostProcess false)
  (Class|WizardsandDragonsCharacter|SetInputEnabled))

(event Custom|ChangeOrbColor_Multicast
  (params (Color :type Linear%20Color%20Structure))
  (bind _returnvalue (Rendering|Material|CreateDynamicMaterialInstance (Variables|Default|GetOrb) 0 "/Game/Meshes/Staff/M_EmissiveOrb.M_EmissiveOrb" "None" :!class /Script/Engine.PrimitiveComponent))
  (Rendering|Material|SetVectorParameterValue _returnvalue "ColorParam" Color :!class /Script/Engine.MaterialInstanceDynamic)
  (Effects|Components|ParticleSystem|SetColorParameter (Variables|Default|GetOrbEffect) "InstancePointColorScaleOverLife" Color)
  (Effects|Components|ParticleSystem|SetColorParameter (Variables|Default|GetOrbEffect) "InstanceSparkleColorScaleOverLife" Color))

(event Custom|ChangeOrbColor
  (params (Color :type Linear%20Color%20Structure))
  (Networking|SwitchHasAuthority
    (:Authority
      (CallFunction|ChangeOrbColorMulticast Color))
    (:Remote
      (CallFunction|ChangeOrbColorServer Color))))

(event Custom|OnResurrectHatAndStaff
  ;[1 1 1] Resurrect HAT & STAFF
  (Cosmetics|ResetHat)
  (Cosmetics|ResetStaff))

(event Custom|ChangeOrbColor_Server
  (params (Color :type Linear%20Color%20Structure))
  (CallFunction|ChangeOrbColorMulticast Color))

(event Custom|HatStaffOnDeathAnimation
  ;[1 1 1] Hat And Staff Stuff
  (bind _successfully_detached (Cosmetics|DetachHat))
  (Cosmetics|AddHatForce _successfully_detached)
  (Cosmetics|DetachStaff))

(event Custom|StartSprint
  (if (Variables|Default|GetCanSprint)
    (Variables|/Script/Engine.CharacterMovementComponent|SetMaxWalkSpeed (Variables|Character|GetCharacterMovement) (Variables|Default|GetSprintMaxSpeed))
    (Utilities|FlowControl|DoOnce false :!label _label
      (:Completed
        (Variables|Default|SetCanSprint false)
        (Utilities|FlowControl|Delay 1.0)
        (CallFunction|StopSprint)
        (Utilities|FlowControl|Delay 5.0)
        (Variables|Default|SetCanSprint true)
        (goto _label Reset)))))

(event Custom|FadeInDeathPostProcess
  (params (FadeIn :type Boolean))
  (if (Pawn|IsLocallyControlled)
    (if FadeIn
      (Variables|/Script/Engine.PostProcessComponent|SetbEnabled (Variables|Default|GetPostProcess) true)
      (bind _newvalue (Timeline|Timeline_0 PlayFromStart)
        (:Update
          (Utilities|Struct|SetmembersinPostProcessSettings (Variables|/Script/Engine.PostProcessComponent|GetSettings (Variables|Default|GetPostProcess)) (Math|Vector4|MakeVector4 _newvalue _newvalue _newvalue _newvalue))))
      (else
        (Utilities|FlowControl|Sequence
          (:then_0
            (Timeline|Timeline_0 ReverseFromEnd))
          (:then_1
            (Utilities|FlowControl|Delay 1.0)
            (Variables|/Script/Engine.PostProcessComponent|SetbEnabled (Variables|Default|GetPostProcess) false)))))))

(event Custom|StopSprint
  (Variables|/Script/Engine.CharacterMovementComponent|SetMaxWalkSpeed (Variables|Character|GetCharacterMovement) (Variables|Default|GetNormalMaxSpeed)))

(event EventOnSpellCast
  (Variables|Default|SetIsCastingSpell true)
  (Utilities|FlowControl|RetriggerableDelay 0.2)
  (Variables|Default|SetIsCastingSpell false))

(event EventSetHat
  (params (HatNumber :type Integer))
  (Variables|Cosmetics|SetIsHatAttached true)
  (Rendering|SetVisibility (Utilities|Select :Index HatNumber :Option%200 (Variables|Default|GetHat2) :Option%201 (Variables|Default|GetHat1)) false false)
  (Transformation|AttachComponentToComponent (Variables|Default|GetHatSocket) (Variables|Character|GetMesh) "head" "SnapToTarget" "KeepWorld" "SnapToTarget" false))

(event EventBeginPlay
  (Utilities|FlowControl|Sequence
    (:then_0
      (Networking|SwitchHasAuthority
        (:Authority
          (Variables|Default|SetOrbColor (Utilities|Select :Index (Variables|/Script/WizardsAndDragons.WADHealthComponent|GetHealthStateEnum (Variables|Default|GetHealthComponent)) :HE_FullHealth "(R=0.187448,G=1.000000,B=0.024608,A=1.000000)" :HE_ThreeQuarterHealth "(R=0.955831,G=1.000000,B=0.000000,A=1.000000)" :HE_HalfHealth "(R=1.000000,G=0.438857,B=0.016962,A=1.000000)" :HE_QuarterHealth "(R=1.000000,G=0.000000,B=0.009744,A=1.000000)" :HE_NoHealth "(R=0.010417,G=0.010417,B=0.010417,A=0.838000)")))))
    (:then_1
      (bind _aswbp_player_health_bar (Utilities|Casting|CastToWBP_PlayerHealthBar (UserInterface|GetUserWidgetObject (Variables|Default|GetHealthBar))))
      (Variables|/Game/Blueprints/WBP_PlayerHealthBar.WBP_PlayerHealthBar_C|SetHealthComp _aswbp_player_health_bar (Variables|Default|GetHealthComponent))
      (UserInterface|Viewport|AddtoViewport (UserInterface|GetUserWidgetObject (Variables|Default|GetGameStateWidget)) 0))))

(event Input|KeyboardEvents|LeftShift
  (params (Key :type Key%20Structure :default "None"))
  (:Pressed
    (if (Pawn|IsLocallyControlled)
      (CallFunction|StartSprint)))
  (:Released
    (if (Pawn|IsLocallyControlled)
      (CallFunction|StopSprint))))

(fn ConstructionScript
  (Utilities|Array|AddUnique (Variables|Default|GetSpellSlots) (Variables|Default|GetFireboltSpell))
  (Utilities|Array|AddUnique (Variables|Default|GetSpellSlots) (Variables|Default|GetFireballSpell))
  (Utilities|Array|AddUnique (Variables|Default|GetSpellSlots) (Variables|Default|GetMageOrbSpell))
  (Utilities|Array|AddUnique (Variables|Default|GetSpellSlots) (Variables|Default|GetResurrectionSpell)))

(fn OnRepOrbColor
  (bind _orbcolor (Variables|Default|GetOrbColor))
  (bind _returnvalue (Rendering|Material|CreateDynamicMaterialInstance (Variables|Default|GetOrb) 0 "/Game/Meshes/Staff/M_EmissiveOrb.M_EmissiveOrb" "None" :!class /Script/Engine.PrimitiveComponent))
  (Rendering|Material|SetVectorParameterValue _returnvalue "ColorParam" _orbcolor :!class /Script/Engine.MaterialInstanceDynamic)
  (Effects|Components|ParticleSystem|SetColorParameter (Variables|Default|GetOrbEffect) "InstancePointColorScaleOverLife" _orbcolor)
  (Effects|Components|ParticleSystem|SetColorParameter (Variables|Default|GetOrbEffect) "InstanceSparkleColorScaleOverLife" _orbcolor))

(fn DetachHat
  (if (Variables|Cosmetics|GetIsHatAttached)
    (Variables|Cosmetics|SetIsHatAttached false)
    (Variables|Cosmetics|SetHatOriginTransform1 (Transformation|GetRelativeTransform (Variables|Default|GetHat1)))
    (Variables|Cosmetics|SetHatOriginTransform2 (Transformation|GetRelativeTransform (Variables|Default|GetHat2)))
    (Collision|SetCollisionEnabled (Variables|Default|GetHat1) "PhysicsOnly")
    (Collision|SetCollisionEnabled (Variables|Default|GetHat2) "PhysicsOnly")
    (Physics|SetSimulatePhysics (Variables|Default|GetHat1) true)
    (Physics|SetSimulatePhysics (Variables|Default|GetHat2) true)
    (return true)
    (else
      (return false))))

(fn ResetHat
  (if (not (Variables|Cosmetics|GetIsHatAttached))
    (Variables|Cosmetics|SetIsHatAttached true)
    (Physics|SetSimulatePhysics (Variables|Default|GetHat1) false)
    (Physics|SetSimulatePhysics (Variables|Default|GetHat2) false)
    (Collision|SetCollisionEnabled (Variables|Default|GetHat1) "NoCollision")
    (Collision|SetCollisionEnabled (Variables|Default|GetHat2) "NoCollision")
    (Transformation|AttachComponentToComponent (Variables|Default|GetHat1) (Variables|Default|GetHatSocket) "None" "KeepWorld" "KeepWorld" "KeepWorld" false)
    (Transformation|AttachComponentToComponent (Variables|Default|GetHat2) (Variables|Default|GetHatSocket) "None" "KeepWorld" "KeepWorld" "KeepWorld" false)
    (Transformation|SetRelativeTransform (Variables|Default|GetHat1) (Variables|Cosmetics|GetHatOriginTransform1) false false)
    (Transformation|SetRelativeTransform (Variables|Default|GetHat2) (Variables|Cosmetics|GetHatOriginTransform2) false false)))

(fn AddHatForce
  (params (CanAddForce :type Boolean))
  (bind _hat1 (Variables|Default|GetHat1))
  (bind _hat2 (Variables|Default|GetHat2))
  (if CanAddForce
    (Physics|AddImpulse _hat1 (Math|Vector|MakeVector (Math|Conversions|ToFloat(Integer) (Math|Random|RandomIntegerinRange -200 200)) (Math|Conversions|ToFloat(Integer) (Math|Random|RandomIntegerinRange -200 200)) 3.5e+02) "None" true)
    (Class|PrimitiveComponent|AddTorqueinRadians _hat1 "100.000000,100.000000, 0" "None" true)
    (Physics|AddImpulse _hat2 (Math|Vector|MakeVector (Math|Conversions|ToFloat(Integer) (Math|Random|RandomIntegerinRange -200 200)) (Math|Conversions|ToFloat(Integer) (Math|Random|RandomIntegerinRange -200 200)) 3.5e+02) "None" true)
    (Class|PrimitiveComponent|AddTorqueinRadians _hat2 "100.000000,100.000000, 0" "None" true)))

(fn ResetStaff
  (Physics|SetSimulatePhysics (Variables|Default|GetStaff) false)
  (Collision|SetCollisionEnabled (Variables|Default|GetStaff) "NoCollision")
  (Transformation|AttachComponentToComponent (Variables|Default|GetStaff) (Variables|Default|GetStaffSocket) "None" "KeepWorld" "KeepWorld" "KeepWorld" false)
  (Transformation|SetRelativeTransform (Variables|Default|GetStaff) (Variables|Cosmetics|GetStaffOriginTransform) false false))

(fn DetachStaff
  (Variables|Cosmetics|SetStaffOriginTransform (Transformation|GetRelativeTransform (Variables|Default|GetStaff)))
  (Collision|SetCollisionEnabled (Variables|Default|GetStaff) "PhysicsOnly")
  (Physics|SetSimulatePhysics (Variables|Default|GetStaff) true))