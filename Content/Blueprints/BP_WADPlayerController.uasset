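; BP_WADPlayerController is a player controller that sets a custom cursor and handles spell targeting and casting.
; On the local controller it builds a spell slot widget for each of OwnedCharacter's spells, retrying on a short delay until that character is valid.
; Slot clicks and five slot input actions toggle SpellTargetSystem for the chosen spell.
; Left mouse casts the spell while targeting is active.
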(event Custom|SpawnWidgets
  (bind _ownedcharacter (Variables|Default|GetOwnedCharacter))
  ;[1 1 1] Create Spell Slot Widgets
  (if (Pawn|IsLocalController)
    (bind _returnvalue (UserInterface|CreateWidget "/Game/Blueprints/UI_Blueprints/WBP_SpellSlots.WBP_SpellSlots_C" self))
    (bind _output_get (Variables|Default|SetSpellSlotsWidget _returnvalue))
    (UserInterface|Viewport|AddtoViewport _output_get 0)
    (Utilities|IsValid _ownedcharacter :!label _label
      (:Is%20Valid
        (for (_array_element _array_index) (Variables|/Script/WizardsAndDragons.WizardsAndDragonsCharacter|GetSpellSlots _ownedcharacter)
          (bind (_success _errormessage _createdspellwidget) (Default|CreateSpellSlotWidget (Variables|Default|GetSpellSlotsWidget) _array_element (+ _array_index 1) self))
          (if _success
            (EventDispatchers|BindEventtoOnSpellClicked _createdspellwidget (delegate Custom|StartSpellTargeting))
            (else
              (Development|PrintText (Utilities|Text|FormatText "Spawn Widgets Error: {0}" _errormessage))))))
      (:Is%20Not%20Valid
        (Utilities|FlowControl|Delay 0.2)
        (goto _label)))))

(event Custom|SpellSlotInput
  (params (SpellSlotIndex :type Integer))
  (bind _spelltargetsystem (Variables|Default|GetSpellTargetSystem))
  (bind _ownedcharacter (Variables|Default|GetOwnedCharacter))
  (bind _spellslots (Variables|/Script/WizardsAndDragons.WizardsAndDragonsCharacter|GetSpellSlots _ownedcharacter))
  (bind _output (Utilities|Array|Get(acopy) _spellslots SpellSlotIndex))
  ;[1 1 1] Spell Slot Input
  (if (Class|SpellTargetSystemComponent|GetIsSystemAlreadyActive (Variables|Default|GetSpellTargetSystem) _output)
    (Class|SpellTargetSystemComponent|StopSpellTargetSystem _spelltargetsystem)
    (else
      (Class|SpellTargetSystemComponent|StartSpellTargetSystem _spelltargetsystem _output))))

(event Custom|StartSpellTargeting
  (params (SpellComponent :type Spell%20Base%20Object%20Reference))
  (bind _spelltargetsystem (Variables|Default|GetSpellTargetSystem))
  ;[1 1 1] Create Spell Slot Widgets
  ;;[1 1 1] Widget Spell Targeting
  (if (Class|SpellTargetSystemComponent|GetIsSystemAlreadyActive (Variables|Default|GetSpellTargetSystem) SpellComponent)
    (Class|SpellTargetSystemComponent|StopSpellTargetSystem _spelltargetsystem)
    (else
      (Class|SpellTargetSystemComponent|StartSpellTargetSystem _spelltargetsystem SpellComponent))))

(event EventBeginPlay
  ;[1 1 1] BeginPlay
  (bind _returnvalue (UserInterface|CreateWidget "/Game/Blueprints/UI_Blueprints/WBP_Cursor.WBP_Cursor_C"))
  (Class|PlayerController|SetMouseCursorWidget "Default" _returnvalue)
  (CallFunction|SpawnWidgets))

(event Input|ActionEvents|InputActionLeftMouseButton
  (params (Key :type Key%20Structure :default "None"))
  ;[1 1 1] Cast Spell input
  (:Pressed
    (if (Class|SpellTargetSystemComponent|GetIsSystemActive (Variables|Default|GetSpellTargetSystem))
      (Class|SpellTargetSystemComponent|CastSpell (Variables|Default|GetSpellTargetSystem)))))

(event Input|ActionEvents|InputActionSpellSlot1
  (params (Key :type Key%20Structure :default "None"))
  ;[1 1 1] Spell Slot Input
  (:Pressed
    (CallFunction|SpellSlotInput)))

(event Input|ActionEvents|InputActionSpellSlot2
  (params (Key :type Key%20Structure :default "None"))
  ;[1 1 1] Spell Slot Input
  (:Pressed
    (CallFunction|SpellSlotInput 1)))

(event Input|ActionEvents|InputActionSpellSlot3
  (params (Key :type Key%20Structure :default "None"))
  ;[1 1 1] Spell Slot Input
  (:Pressed
    (CallFunction|SpellSlotInput 2)))

(event Input|ActionEvents|InputActionSpellSlot4
  (params (Key :type Key%20Structure :default "None"))
  ;[1 1 1] Spell Slot Input
  (:Pressed
    (CallFunction|SpellSlotInput 3)))

(event Input|ActionEvents|InputActionSpellSlot5
  (params (Key :type Key%20Structure :default "None"))
  ;[1 1 1] Spell Slot Input
  (:Pressed
    (CallFunction|SpellSlotInput 4)))

(fn ConstructionScript)