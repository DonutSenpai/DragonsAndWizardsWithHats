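; BP_WADGameMode is a game mode that registers AI spawners and player characters, then starts a round-based game.
; On BeginPlay it adds every AISpawner and, nested inside that loop, every BP_WADPlayerCharacter, so players are re-added once per spawner.
; A one-second delay then leads into BeginNewRound.
; Tick prints the current Score on screen each frame as a debug readout.
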(event EventTick
  (params (DeltaSeconds :type Float%20%28single-precision%29))
  (Development|PrintString (Utilities|String|ToString(Text) (Utilities|Text|FormatText "Score: {0} " (Variables|Default|GetScore))) true true "(R=0.000000,G=0.660000,B=1.000000,A=1.000000)" DeltaSeconds))

(event EventBeginPlay
  (Utilities|FlowControl|Sequence
    (:then_0
      (bind _outactors (Actor|GetAllActorsOfClass "/Script/WizardsAndDragons.AISpawner"))
      (for _array_element _outactors
        (Class|WizardsandDragonsGameMode|AddSpawner _array_element)
        (bind _outactors_2 (Actor|GetAllActorsOfClass "/Game/Blueprints/BP_WADPlayerCharacter.BP_WADPlayerCharacter_C"))
        (for _array_element_2 _outactors_2
          (Class|WizardsandDragonsGameMode|AddPlayer _array_element_2))))
    (:then_1
      (Utilities|FlowControl|Delay 1.0)
      (Class|WizardsandDragonsGameMode|BeginNewRound))))

(fn ConstructionScript)