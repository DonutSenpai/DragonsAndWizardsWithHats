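; BP_FireboltEffect is a firebolt effect actor that flies to a target, then spawns a half-scale hit particle and destroys itself.
; ShootFirebolt uses timelines to lerp from its start point, following a valid target actor's live position or else a fixed location, scaled by TravelTime.
; ShootAFirebolt is a simpler variant that lerps from the current position each update toward a location.
; Movement teleports nothing and uses no sweep, so arrival is timeline-driven, not collision-driven.
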(event Custom|ShootFirebolt
  (params (TravelTime :type Float%20%28single-precision%29) (TargetLocation :type Vector) (TargetActor :type Actor%20Object%20Reference))
  (Variables|Default|SetStartLocation (Transformation|GetActorLocation))
  (Utilities|IsValid TargetActor
    (:Is%20Valid
      (Variables|Default|SetTargetActor TargetActor)
      (bind _newtrack_0 (Timeline|Timeline_1 PlayFromStart)
        (:Update
          (Transformation|SetActorLocation (Math|Vector|Lerp(Vector) (Variables|Default|GetStartLocation) (Transformation|GetActorLocation (Variables|Default|GetTargetActor)) (/ _newtrack_0 TravelTime)) false false)
          (if (>= (/ _newtrack_0 TravelTime) TravelTime)
            (CallFunction|Explode)))
        (:Finished
          (CallFunction|Explode))))
    (:Is%20Not%20Valid
      (Variables|Default|SetTargetLocation TargetLocation)
      (bind _newtrack_0_2 (Timeline|Timeline_2 PlayFromStart)
        (:Update
          (Transformation|SetActorLocation (Math|Vector|Lerp(Vector) (Variables|Default|GetStartLocation) (Variables|Default|GetTargetLocation) (/ _newtrack_0_2 TravelTime)) false false)
          (if (>= (/ _newtrack_0_2 TravelTime) TravelTime)
            (CallFunction|Explode)))))))

(event Custom|Explode
  ;[1 1 1] Explode
  (Effects|SpawnEmitteratLocation (Variables|Default|GethitFx) (Transformation|GetActorLocation) "0, 0, 0" "0.500000,0.500000,0.500000")
  (Actor|DestroyActor))

(event Custom|ShootAFirebolt
  (params (TargetLocation :type Vector))
  (bind _newtrack_0 (Timeline|Timeline_0 PlayFromStart)
    (:Update
      (Transformation|SetActorLocation (Math|Vector|Lerp(Vector) (Transformation|GetActorLocation) TargetLocation _newtrack_0) false false))
    (:Finished
      (CallFunction|Explode))))

(fn ConstructionScript)