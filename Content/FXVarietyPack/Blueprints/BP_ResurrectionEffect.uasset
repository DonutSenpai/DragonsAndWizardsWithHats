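; Resurrection effect actor that flies from its spawn location to a target actor and plays a hit effect on arrival.
; ShootResurrectBall drives a timeline that lerps toward the target's live location, then shrinks the FX1 component.
; At full alpha, EndEffect spawns the hit emitter below the actor, scales it to zero and destroys both.
; TravelTime is stored but never applied to the timeline, and no revive logic runs here.
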(event Custom|ShootResurrectBall
  (params (TravelTime :type Float%20%28single-precision%29) (TargetActor :type Actor%20Object%20Reference))
  (Variables|Default|SetTravelTime TravelTime)
  (Variables|Default|SetTargetActor TargetActor)
  (Variables|Default|SetStartLocation (Transformation|GetActorLocation))
  (bind _alpha (Timeline|Timeline_2 PlayFromStart)
    (:Update
      (Transformation|SetActorLocation (Math|Vector|Lerp(Vector) (Variables|Default|GetStartLocation) (Transformation|GetActorLocation (Variables|Default|GetTargetActor)) _alpha) false false)
      (if (>= _alpha 1.0)
        (CallFunction|EndEffect)))
    (:Finished
      (bind _alpha_2 (Timeline|DiminishEffect Play)
        (:Update
          (Transformation|SetWorldScale3D (Variables|Default|GetFX1) (Math|Vector|Lerp(Vector) "0.750000,0.750000,0.750000" "0, 0, 0" _alpha_2)))))))

(event Custom|EndEffect
  ;[1 1 1] EndEffect
  (bind _returnvalue (Effects|SpawnEmitteratLocation (Variables|Default|GethitFx) (- (Transformation|GetActorLocation) "0, 0,96.000000")))
  (Variables|Default|SetHealEffect _returnvalue)
  (bind _alpha (Timeline|DiminishOtherEffect PlayFromStart)
    (:Update
      (Transformation|SetWorldScale3D (Variables|Default|GetHealEffect) (Math|Vector|Lerp(Vector) "1.000000,1.000000,1.000000" "0, 0, 0" _alpha)))
    (:Finished
      (Components|DestroyComponent (Variables|Default|GetHealEffect))
      (Actor|DestroyActor))))

(fn ConstructionScript)