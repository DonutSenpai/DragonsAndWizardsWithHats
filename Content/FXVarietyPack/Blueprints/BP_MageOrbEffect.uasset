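; Mage orb projectile effect actor that flies from its spawn point to a target location, then shrinks and bursts.
; ShootMageOrb flattens the target to the orb's height and moves it there by timeline lerp; the stored TravelTime is unused here.
; On arrival, ExitEffect scales both FX components toward zero before destruction, while a delayed branch spawns the hit emitter and disables collision.
; A separate overlap event attaches a water-ball hit emitter to the given actor.
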(event Custom|ShootMageOrb
  (params (TravelTime :type Float%20%28single-precision%29) (TargetLocation :type Vector))
  ;[1 1 1] Shoot The Orb!
  (Variables|Default|SetTravelTime TravelTime)
  (Variables|Default|SetTargetLocation (Math|Vector|MakeVector (.x TargetLocation) (.y TargetLocation) (.z (Transformation|GetActorLocation))))
  (Variables|Default|SetStartLocation (Transformation|GetActorLocation))
  ;;[1 1 1] at Location
  (bind (_direction _newtrack_0 _heightadjustmentalpha) (Timeline|Timeline_2 PlayFromStart)
    (:Update
      (Transformation|SetActorLocation (Math|Vector|Lerp(Vector) (Variables|Default|GetStartLocation) (Variables|Default|GetTargetLocation) _newtrack_0) false false)
      (Transformation|SetWorldLocation (Variables|Default|GetFX1) (Math|Vector|Lerp(Vector) (Variables|Default|GetStartLocation) (Variables|Default|GetTargetLocation) _newtrack_0) false false)
      (if (>= _newtrack_0 1.0)
        (CallFunction|ExitEffect)))))

(event Custom|Explode
  ;[1 1 1] Explode
  (Effects|SpawnEmitteratLocation (Variables|Default|GethitFx) (Transformation|GetActorLocation) "0, 0, 0" "0.250000,0.250000,0.250000"))

(event Custom|ExitEffect
  (bind _fx1 (Variables|Default|GetFX1))
  (bind _fx2 (Variables|Default|GetFX2))
  (Utilities|FlowControl|Sequence
    (:then_0
      (bind _alpha (Timeline|DiminishEffect Play)
        (:Update
          (Transformation|SetWorldScale3D _fx1 (Math|Vector|Lerp(Vector) (Transformation|GetWorldScale _fx1) "0, 0, 0" _alpha))
          (Transformation|SetWorldScale3D _fx2 (Math|Vector|Lerp(Vector) (Transformation|GetWorldScale _fx2) "0, 0, 0" _alpha)))
        (:Finished
          (Actor|DestroyActor))))
    (:then_1
      (Utilities|FlowControl|Delay 0.2)
      (CallFunction|Explode)
      (Collision|SetCollisionEnabled (Variables|Default|GetMageOrbCollision) "NoCollision"))))

(event EventBeginPlay
  (Components|Sphere|SetSphereRadius (Variables|Default|GetMageOrbCollision) (Variables|Default|GetRadius) true))

(event EventOnMageOrbOverlapEffect
  (params (OverlappedActor :type Actor%20Object%20Reference))
  (Effects|SpawnEmitterAttached "/Game/FXVarietyPack/Particles/P_ky_waterBallHit.P_ky_waterBallHit" (Variables|/Script/Engine.Actor|GetRootComponent OverlappedActor) "None" "0, 0, 0" "0, 0, 0" "0.500000,0.500000,0.500000"))

(fn ConstructionScript)