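; BP_FireballEffect is a fireball effect actor that travels in an arc to a target location and explodes.
; ShootFireball stores the travel parameters and starts a timeline that lerps from the start to the target, adding a curve-driven vertical offset without sweeping.
; The stored TravelTime is not read in this graph.
; When the travel alpha completes, Explode spawns the hit emitter and destroys the actor.
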(event Custom|ShootFireball
  (params (TravelTime :type Float%20%28single-precision%29) (TargetLocation :type Vector))
  ;[1 1 1] Shoot The Fireball!
  (Variables|Default|SetTravelTime TravelTime)
  (Variables|Default|SetTargetLocation TargetLocation)
  (Variables|Default|SetStartLocation (Transformation|GetActorLocation))
  ;;[1 1 1] Fireball at Location
  (bind (_direction _newtrack_0 _heightadjustmentalpha) (Timeline|Timeline_2 PlayFromStart)
    (:Update
      (Transformation|SetActorLocation (+ (Math|Vector|Lerp(Vector) (Variables|Default|GetStartLocation) (Variables|Default|GetTargetLocation) _newtrack_0) (* "0, 0,200.000000" _heightadjustmentalpha)) false false)
      (if (>= _newtrack_0 1.0)
        (CallFunction|Explode)))))

(event Custom|Explode
  ;[1 1 1] Explode
  (Effects|SpawnEmitteratLocation (Variables|Default|GethitFx) (Transformation|GetActorLocation) "0, 0, 0" "1.500000,1.500000,1.500000")
  (Actor|DestroyActor))

(fn ConstructionScript)