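; BP_FireStorm is a boss dragon fire storm effect actor that plays a timed two-stage visual sequence.
; On begin play it activates a magic circle effect for an initial delay, then deactivates it and runs the fire storm effect for a set duration.
; After the storm deactivates, it waits briefly before destroying itself.
; The construction script pushes a configurable color to the magic circle effect's color parameter.
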(event Custom|StartFireStormEvent
  (Components|Activation|Activate (Variables|Default|GetFireStormFX) false)
  ;[1 1 1] effect duration control
  (Utilities|FlowControl|Delay (Variables|Default|Getduration))
  ;[1 1 1] effect finish
  (Components|Activation|Deactivate (Variables|Default|GetFireStormFX))
  (Utilities|FlowControl|Delay 3.0)
  ;[1 1 1] effect delete
  (Actor|DestroyActor))

(event EventBeginPlay
  (Components|Activation|Activate (Variables|Default|GetMagicCircleFX) false)
  ;[1 1 1] effect duration control
  (Utilities|FlowControl|Delay (Variables|Default|GetInitialDelay))
  ;[1 1 1] effect finish
  (Components|Activation|Deactivate (Variables|Default|GetMagicCircleFX))
  (CallFunction|StartFireStormEvent))

(fn ConstructionScript
  (|CallParentFunction)
  (Effects|Components|ParticleSystem|SetVectorParameter (Variables|Default|GetMagicCircleFX) "color" (Math|Conversions|ToVector(LinearColor) (Variables|Default|Getcolor))))