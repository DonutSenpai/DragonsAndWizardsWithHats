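; Boss dragon actor that deals melee damage to the player and tracks its own health.
; Head and claw collision overlaps damage the player's WADHealthComponent and launch them along the dragon's forward vector, with the head hurting more and claws pushing harder.
; OnResetMelee disables all three hitboxes, which are also deactivated on BeginPlay.
; Its health component feeds the boss health bar widget and reports damage events with the instigator.
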(event OnComponentBeginOverlap(LeftClawCollision)
  (params (OverlappedComponent :type Primitive%20Component%20Object%20Reference) (OtherActor :type Actor%20Object%20Reference) (OtherComp :type Primitive%20Component%20Object%20Reference) (OtherBodyIndex :type Integer) (bFromSweep :type Boolean) (SweepResult :type Hit%20Result%20Structure%20%28by%20ref%29))
  (bind _asbp_wadplayer_character (Utilities|Casting|CastToBP_WADPlayerCharacter OtherActor))
  (if (Utilities|IsValid (Actor|GetComponentbyClass _asbp_wadplayer_character "/Script/WizardsAndDragons.WADHealthComponent"))
    (Class|WADHealthComponent|DecreaseHealth (Actor|GetComponentbyClass _asbp_wadplayer_character "/Script/WizardsAndDragons.WADHealthComponent") 25.0 self)
    (Character|LaunchCharacter _asbp_wadplayer_character (* (Transformation|GetActorForwardVector) 3e+03) false false)))

(event OnComponentBeginOverlap(RightClawCollision)
  (params (OverlappedComponent :type Primitive%20Component%20Object%20Reference) (OtherActor :type Actor%20Object%20Reference) (OtherComp :type Primitive%20Component%20Object%20Reference) (OtherBodyIndex :type Integer) (bFromSweep :type Boolean) (SweepResult :type Hit%20Result%20Structure%20%28by%20ref%29))
  (bind _asbp_wadplayer_character (Utilities|Casting|CastToBP_WADPlayerCharacter OtherActor))
  (if (Utilities|IsValid (Actor|GetComponentbyClass _asbp_wadplayer_character "/Script/WizardsAndDragons.WADHealthComponent"))
    (Class|WADHealthComponent|DecreaseHealth (Actor|GetComponentbyClass _asbp_wadplayer_character "/Script/WizardsAndDragons.WADHealthComponent") 25.0 self)
    (Character|LaunchCharacter _asbp_wadplayer_character (* (Transformation|GetActorForwardVector) 3e+03) false false)))

(event OnComponentBeginOverlap(HeadCollision)
  (params (OverlappedComponent :type Primitive%20Component%20Object%20Reference) (OtherActor :type Actor%20Object%20Reference) (OtherComp :type Primitive%20Component%20Object%20Reference) (OtherBodyIndex :type Integer) (bFromSweep :type Boolean) (SweepResult :type Hit%20Result%20Structure%20%28by%20ref%29))
  (bind _asbp_wadplayer_character (Utilities|Casting|CastToBP_WADPlayerCharacter OtherActor))
  (if (Utilities|IsValid (Actor|GetComponentbyClass _asbp_wadplayer_character "/Script/WizardsAndDragons.WADHealthComponent"))
    (Class|WADHealthComponent|DecreaseHealth (Actor|GetComponentbyClass _asbp_wadplayer_character "/Script/WizardsAndDragons.WADHealthComponent") 5e+01 self)
    (Character|LaunchCharacter _asbp_wadplayer_character (* (Transformation|GetActorForwardVector) 1.5e+03) false false)))

(event OnHealthChanged(HealthComp)
  (params (ChangeValue :type Float%20%28single-precision%29) (InstigatingActor :type Actor%20Object%20Reference))
  (Class|AISenseDamage|ReportDamageEvent self InstigatingActor ChangeValue "0, 0, 0"))

(event EventBeginPlay
  (bind _aswbp_boss_dragon_health_bar (Utilities|Casting|CastToWBP_BossDragonHealthBar (UserInterface|GetUserWidgetObject (Variables|Default|GetBossDragonHealthbar))))
  (Variables|/Game/AI/Widgets/WBP_BossDragonHealthBar.WBP_BossDragonHealthBar_C|SetHealthComp _aswbp_boss_dragon_health_bar (Variables|Default|GetHealthComp))
  (Components|Activation|Deactivate (Variables|Default|GetHeadCollision))
  (Components|Activation|Deactivate (Variables|Default|GetLeftClawCollision))
  (Components|Activation|Deactivate (Variables|Default|GetRightClawCollision)))

(event EventOnResetMelee
  (Collision|SetCollisionEnabled (Variables|Default|GetLeftClawCollision) "NoCollision")
  (Collision|SetCollisionEnabled (Variables|Default|GetRightClawCollision) "NoCollision")
  (Collision|SetCollisionEnabled (Variables|Default|GetHeadCollision) "NoCollision"))

(fn ConstructionScript)