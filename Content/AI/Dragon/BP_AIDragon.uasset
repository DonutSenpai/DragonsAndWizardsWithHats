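; BP_AIDragon is an AI dragon enemy that damages and knocks back the player with claw attacks.
; Each claw collision overlap with the player character lowers its health component and launches it along the dragon's forward vector.
; A melee reset event disables both claw collisions.
; Health changes report damage events for AI sensing, and BeginPlay links the health component to a dragon health bar widget.
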(event OnComponentBeginOverlap(LeftClawCollision)
  (params (OverlappedComponent :type Primitive%20Component%20Object%20Reference) (OtherActor :type Actor%20Object%20Reference) (OtherComp :type Primitive%20Component%20Object%20Reference) (OtherBodyIndex :type Integer) (bFromSweep :type Boolean) (SweepResult :type Hit%20Result%20Structure%20%28by%20ref%29))
  (bind _asbp_wadplayer_character (Utilities|Casting|CastToBP_WADPlayerCharacter OtherActor))
  (if (Utilities|IsValid (Actor|GetComponentbyClass _asbp_wadplayer_character "/Script/WizardsAndDragons.WADHealthComponent"))
    (Class|WADHealthComponent|DecreaseHealth (Actor|GetComponentbyClass _asbp_wadplayer_character "/Script/WizardsAndDragons.WADHealthComponent") 25.0 self)
    (Character|LaunchCharacter _asbp_wadplayer_character (* (Transformation|GetActorForwardVector) 2e+03) false false)))

(event OnComponentBeginOverlap(RightClawCollision)
  (params (OverlappedComponent :type Primitive%20Component%20Object%20Reference) (OtherActor :type Actor%20Object%20Reference) (OtherComp :type Primitive%20Component%20Object%20Reference) (OtherBodyIndex :type Integer) (bFromSweep :type Boolean) (SweepResult :type Hit%20Result%20Structure%20%28by%20ref%29))
  (bind _asbp_wadplayer_character (Utilities|Casting|CastToBP_WADPlayerCharacter OtherActor))
  (if (Utilities|IsValid (Actor|GetComponentbyClass _asbp_wadplayer_character "/Script/WizardsAndDragons.WADHealthComponent"))
    (Class|WADHealthComponent|DecreaseHealth (Actor|GetComponentbyClass _asbp_wadplayer_character "/Script/WizardsAndDragons.WADHealthComponent") 25.0 self)
    (Character|LaunchCharacter _asbp_wadplayer_character (* (Transformation|GetActorForwardVector) 2e+03) false false)))

(event OnHealthChanged(HealthComp)
  (params (ChangeValue :type Float%20%28single-precision%29) (InstigatingActor :type Actor%20Object%20Reference))
  (Class|AISenseDamage|ReportDamageEvent self InstigatingActor ChangeValue "0, 0, 0"))

(event EventBeginPlay
  (bind _aswbp_dragon_health_bar (Utilities|Casting|CastToWBP_DragonHealthBar (UserInterface|GetUserWidgetObject (Variables|Default|GetDragonHeathBar))))
  (Variables|/Game/AI/Widgets/WBP_DragonHealthBar.WBP_DragonHealthBar_C|SetHealthComp _aswbp_dragon_health_bar (Variables|Default|GetHealthComp)))

(event EventOnResetMelee
  (Collision|SetCollisionEnabled (Variables|Default|GetLeftClawCollision) "NoCollision")
  (Collision|SetCollisionEnabled (Variables|Default|GetRightClawCollision) "NoCollision"))

(fn ConstructionScript)